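; BP_FloorSwitch is a floor switch that opens and closes its target sliding doors as something enters or leaves its trigger.
; Overlap sets IsPressed and plays or reverses a Timeline that moves the switch model.
; A DoOnce on the Timeline update, reset on finish, plays the sound and opens or closes every TargetActor door according to IsPressed.
; StayPressed only reaches an empty DoOnce, so releasing always reverses the switch.
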(event `self.SwitchTrigger.OnComponentBeginOverlap`
  (params (OverlappedComponent :type "PrimitiveComponent Object Reference") (OtherActor :type "Actor Object Reference") (OtherComp :type "PrimitiveComponent Object Reference") (OtherBodyIndex :type Integer) (bFromSweep :type Boolean) (SweepResult :type "HitResult Structure (by ref)"))
  (bind _switchmodel (`self.SwitchModel`))
  (bind _targetactor (`self.targetActor`))
  ;[1 0.5583 0.2582] Checks if button is pressed
  (if (not (`self.isPressed`))
    (set `self.isPressed` true)
    ;[1 0.5583 0.2582] Play Button Press Sound and move switch down to show it activated.
    (bind (_direction _switch) (`Timeline|Timeline_0` :!label _label)
      (:`Update`
        (`SceneComponent.K2_SetRelativeLocation` _switchmodel (`KismetMathLibrary.MakeVector` 0.0 0.0 _switch) false false)
        (`/Engine/EditorBlueprintResources/StandardMacros.DoOnce` false :!label _label_2
          (:`Completed`
            (`GameplayStatics.SpawnSoundAtLocation` "/Game/__Sound/SwitchActivated.SwitchActivated" (`SceneComponent.K2_GetComponentLocation` _switchmodel) (struct) 0.5 1.0 0.0 null null)
            ;[1 0.5583 0.2582] Get Target Actor array and activate
            (if (`self.stayPressed`)
              (`/Engine/EditorBlueprintResources/StandardMacros.DoOnce` false
                (:`Completed`
                  _)))
            (if (`self.isPressed`)
              (for _array_element _targetactor
                (`/Game/__Blueprints/BP_Moveable.Slide Door Open` _array_element))
              (else
                (for _array_element_2 _targetactor
                  (`/Game/__Blueprints/BP_Moveable.Slide Door Closed` _array_element_2)))))))
      (:`Finished`
        (goto _label_2 :!via `Reset`)))))

(event `self.SwitchTrigger.OnComponentEndOverlap`
  (params (OverlappedComponent :type "PrimitiveComponent Object Reference") (OtherActor :type "Actor Object Reference") (OtherComp :type "PrimitiveComponent Object Reference") (OtherBodyIndex :type Integer))
  ;[1 0.5583 0.2582] Checks if button is pressed
  (set `self.isPressed` false)
  (goto _label :!via `Reverse`))

(fn `UserConstructionScript`)