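; BP_1mCube is a physics cube that plays a rock impact sound when it collides hard enough.
; On Hit, it compares its linear velocity with the last stored value and requires a large enough change.
; While the first-person character holds any object, a second, higher threshold against a separate stored velocity applies.
; The sound plays at world origin, and Tick repeatedly wakes the rigid body after a short Delay to prevent freezing.
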(event `self.ReceiveHit`
  (params (MyComp :type "PrimitiveComponent Object Reference") (Other :type "Actor Object Reference") (OtherComp :type "PrimitiveComponent Object Reference") (bSelfMoved :type Boolean) (HitLocation :type "Vector Structure") (HitNormal :type "Vector Structure") (NormalImpulse :type "Vector Structure") (Hit :type "HitResult Structure (by ref)"))
  ;[1 1 1] Gets velocity of the object and if it is above a set number then play a sound when colliding with other objects
  (bind _returnvalue (`PrimitiveComponent.GetPhysicsLinearVelocity` (`self.Cube`) "None"))
  (if (> (`KismetMathLibrary.VSize` (- _returnvalue (`self.LasVel`))) 150.0)
    (set `self.LasVel` _returnvalue)
    ;[1 1 1] Get velocity of object while player is holding and play a sound when colliding
    (bind _asbp_first_person_character (cast `/Game/FirstPerson/Blueprints/BP_FirstPersonCharacter` (`GameplayStatics.GetPlayerCharacter` 0)))
    (if (`/Game/FirstPerson/Blueprints/BP_FirstPersonCharacter.isHoldingObject?` _asbp_first_person_character)
      (bind _returnvalue_2 (`PrimitiveComponent.GetPhysicsLinearVelocity` (`self.Cube`) "None"))
      (if (> (`KismetMathLibrary.VSize` (- _returnvalue_2 (`self.HoldingVel`))) 250.0)
        (set `self.HoldingVel` _returnvalue_2)
        (`GameplayStatics.PlaySoundAtLocation` "/Game/__Sound/RockImpact.RockImpact" (0.0 0.0 0.0) (struct) 1.0 1.0 0.0 null null null null :!label _label))
      (else
        (goto _label)))))

(event `self.ReceiveTick`
  (params (DeltaSeconds :type "Float (single-precision)"))
  ;[1 1 1] Prevents Object from freezing
  (`KismetSystemLibrary.Delay` (+ DeltaSeconds 0.1))
  (`PrimitiveComponent.WakeRigidBody` (`self.Cube`) "None"))

(fn `UserConstructionScript`)